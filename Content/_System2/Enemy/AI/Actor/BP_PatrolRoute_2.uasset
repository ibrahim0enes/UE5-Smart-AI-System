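; BP_PatrolRoute_2 is a patrol route actor for enemy AI, built on a PatrolRoute spline.
; NextPoint steps PointIndex by Direction and flips Direction at the last and first spline points, producing a back-and-forth patrol rather than a loop.
; GetSplinePointWorldLocation returns the world-space location of the current point.
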(event `Next Point`
  (bind _output_get (set `self.Point Index` (+ (`self.Point Index`) (`self.Direction`))))
  (if (== _output_get (- (`SplineComponent.GetNumberOfSplinePoints` (`self.Patrol Route`)) 1))
    (set `self.Direction` -1)
    (elif (== (`self.Point Index`) 0)
      (set `self.Direction` 1))))

(fn `GetSplinePointWorldLocation`
  (returns (Location :type "Vector Structure"))
  (return (`SplineComponent.GetLocationAtSplinePoint` (`self.Patrol Route`) (`self.Point Index`) "World")))

(fn `UserConstructionScript`)