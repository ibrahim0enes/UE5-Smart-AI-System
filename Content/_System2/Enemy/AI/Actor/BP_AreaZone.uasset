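; BP_AreaZone is a box trigger volume that marks an area with an access level for the player's disguise messaging.
; On BeginPlay it shows its AccessLevel on a TextRender.
; When BP_Player2 enters the box it passes AccessLevel to SetDisguiseMessage, and on exit it passes a fixed enum value instead.
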(event `self.ReceiveBeginPlay`
  (`TextRenderComponent.K2_SetText` (`self.TextRender`) (`|GenericToText` (`self.AccessLevel`))))

(event `self.Box.OnComponentBeginOverlap`
  (params (OverlappedComponent :type "PrimitiveComponent Object Reference") (OtherActor :type "Actor Object Reference") (OtherComp :type "PrimitiveComponent Object Reference") (OtherBodyIndex :type Integer) (bFromSweep :type Boolean) (SweepResult :type "HitResult Structure (by ref)"))
  (bind _asbp_player_2 (cast `/Game/_System2/Player/BP_Player2` OtherActor))
  (message `/Game/_System2/Enemy/AI/BPI/BPI_AI.SetDisguise` _asbp_player_2 (`self.AccessLevel`)))

(event `self.Box.OnComponentEndOverlap`
  (params (OverlappedComponent :type "PrimitiveComponent Object Reference") (OtherActor :type "Actor Object Reference") (OtherComp :type "PrimitiveComponent Object Reference") (OtherBodyIndex :type Integer))
  (bind _asbp_player_2 (cast `/Game/_System2/Player/BP_Player2` OtherActor))
  (message `/Game/_System2/Enemy/AI/BPI/BPI_AI.SetDisguise` _asbp_player_2 "NewEnumerator3"))

(fn `UserConstructionScript`)