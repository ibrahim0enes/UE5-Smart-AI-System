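; BP_PatrolRoute is a patrol path for AI, defined by the points of its PatrolRoute spline.
; NextPoint steps PatrolIndex by a direction value that flips at the first and last spline points, so the route ping-pongs instead of looping.
; GetSplinePointWorldLocation returns the world position of the current point.
; The route itself holds the index and direction state.
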(event `Next Point`
  (bind _output_get (set `self.PatrolIndex` (+ (`self.PatrolIndex`) (`self.Directioon`))))
  (if (== _output_get (- (`SplineComponent.GetNumberOfSplinePoints` (`self.PatrolRoute`)) 1))
    (set `self.Directioon` -1)
    (elif (== (`self.PatrolIndex`) 0)
      (set `self.Directioon` 1))))

(fn `GetSplinePointWorldLocation`
  (returns (ReturnValue :type "Vector Structure"))
  (return (`SplineComponent.GetLocationAtSplinePoint` (`self.PatrolRoute`) (`self.PatrolIndex`) "World")))

(fn `UserConstructionScript`)